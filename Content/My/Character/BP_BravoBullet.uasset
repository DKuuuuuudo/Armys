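; BP_BravoBullet is a team-aware bullet that damages enemy characters and credits the kill.
; On Hit, an opposing-team MyCharacter takes damage, gets a Japanese "defeated by" DeathLog from the bullet's Name unless it equals Temp, and, if not already dead, increments the bullet's PlayerState KillNum.
; The bullet is destroyed on any MyCharacter or BP_AlfaBullet hit, while other surfaces destroy it on the second hit.
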(event `self.ReceiveHit`
  (params (MyComp :type "PrimitiveComponent Object Reference") (Other :type "Actor Object Reference") (OtherComp :type "PrimitiveComponent Object Reference") (bSelfMoved :type Boolean) (HitLocation :type "Vector Structure") (HitNormal :type "Vector Structure") (NormalImpulse :type "Vector Structure") (Hit :type "HitResult Structure (by ref)"))
  (bind _name (`self.Name`))
  (bind _playerstate (`self.PlayerState`))
  (bind _asmy_character (cast `/Game/My/Character/MyCharacter` Other)
    (:`then`
      (bind _myplayerstate (`/Game/My/Character/MyCharacter.MyPlayerState` _asmy_character))
      (if (!= (`/Game/My/Class/Main/MyPlayerState.TeamId` _myplayerstate) (`self.TeamID`))
        (if (not (`KismetTextLibrary.EqualEqual_TextText` _name (`self.Temp`)))
          (set `/Game/My/Class/Main/MyPlayerState.DeathLog` (`KismetTextLibrary.Conv_StringToText` (`KismetStringLibrary.Concat_StrStr` (`KismetTextLibrary.Conv_TextToString` _name) "に倒された...")) _myplayerstate))
        (if (not (`/Game/My/Class/Main/MyPlayerState.isDeath` _myplayerstate))
          (bind _result (`/Engine/EditorBlueprintResources/StandardMacros.IncrementInt` (`/Game/My/Class/Main/MyPlayerState.KillNum` _playerstate))
            (:`  `
              (set `/Game/My/Class/Main/MyPlayerState.KillNum` _result _playerstate))))
        (`GameplayStatics.ApplyDamage` Other 1.0)
        (`self.K2_DestroyActor`)
        (else
          (`self.K2_DestroyActor`))))
    (:`CastFailed`
      (cast `/Game/My/Character/BP_AlfaBullet` Other
        (:`then`
          (`self.K2_DestroyActor`))
        (:`CastFailed`
          (bind _result_2 (`/Engine/EditorBlueprintResources/StandardMacros.IncrementInt` (`self.HitNum`))
            (:`  `
              (bind _output_get (set `self.HitNum` _result_2))
              (if (== _output_get 2)
                (`self.K2_DestroyActor`)))))))))

(fn `UserConstructionScript`)