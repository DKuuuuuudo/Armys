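; BP_BravoExplosion is a short-lived explosion actor that damages opposing-team characters and credits kills to its owning player state.
; On spawn, the Ball grows in steps through a delayed recursive event, and the actor self-destructs after a brief lifetime.
; Overlapping an enemy MyCharacter writes the victim's death log, increments KillNum if the victim is still alive, and applies damage.
; Any overlap destroys the explosion, including teammates and non-characters.
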(event `self.ReceiveActorBeginOverlap`
  (params (OtherActor :type "Actor Object Reference"))
  (bind _name (`self.Name`))
  (bind _playerstate (`self.PlayerState`))
  (bind _asmy_character (cast `/Game/My/Character/MyCharacter` OtherActor)
    (:`then`
      (bind _myplayerstate (`/Game/My/Character/MyCharacter.MyPlayerState` _asmy_character))
      (if (!= (`/Game/My/Class/Main/MyPlayerState.TeamId` _myplayerstate) (`self.TeamID`))
        (if (not (`KismetTextLibrary.EqualEqual_TextText` _name (`self.Temp`)))
          (set `/Game/My/Class/Main/MyPlayerState.DeathLog` (`KismetTextLibrary.Conv_StringToText` (`KismetStringLibrary.Concat_StrStr` (`KismetTextLibrary.Conv_TextToString` _name) "に倒された...")) _myplayerstate))
        (if (not (`/Game/My/Class/Main/MyPlayerState.isDeath` _myplayerstate))
          (bind _result (`/Engine/EditorBlueprintResources/StandardMacros.IncrementInt` (`/Game/My/Class/Main/MyPlayerState.KillNum` _playerstate))
            (:`  `
              (set `/Game/My/Class/Main/MyPlayerState.KillNum` _result _playerstate))))
        (`GameplayStatics.ApplyDamage` OtherActor 1.0)
        (`self.K2_DestroyActor`)
        (else
          (`self.K2_DestroyActor`))))
    (:`CastFailed`
      (`self.K2_DestroyActor`))))

(event `self.ReceiveBeginPlay`
  (`SceneComponent.SetRelativeScale3D` (`self.Ball`) (0.5 0.5 0.5))
  (`self.ExplosionScale` false)
  (`KismetSystemLibrary.Delay` 0.3)
  (`/Engine/EditorBlueprintResources/StandardMacros.IsValid` self
    (:`Is Valid`
      (`self.K2_DestroyActor`))))

(event `ExplosionScale`
  (params (Flag :type Boolean))
  (bind _returnvalue (+ (`SceneComponent.RelativeScale3D` (`self.Ball`)) (0.2 0.2 0.2)))
  (if (not Flag)
    (`KismetSystemLibrary.Delay` 0.03)
    (`SceneComponent.SetRelativeScale3D` (`self.Ball`) _returnvalue)
    (`self.ExplosionScale` (== _returnvalue (1.7 1.7 1.7) :`ErrorTolerance` 0.1))))

(fn `UserConstructionScript`)