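; BP_Bullet is a projectile actor that damages any MyCharacter it hits.
; Its Hit event applies a fixed damage to the character and destroys the bullet, or just destroys it when the other actor is also a BP_Bullet.
; Any other impact increments HitNum, and the bullet is destroyed on the second such hit, so it survives one impact with other objects.
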(event `self.ReceiveHit`
  (params (MyComp :type "PrimitiveComponent Object Reference") (Other :type "Actor Object Reference") (OtherComp :type "PrimitiveComponent Object Reference") (bSelfMoved :type Boolean) (HitLocation :type "Vector Structure") (HitNormal :type "Vector Structure") (NormalImpulse :type "Vector Structure") (Hit :type "HitResult Structure (by ref)"))
  (cast `/Game/My/Character/MyCharacter` Other
    (:`then`
      (`GameplayStatics.ApplyDamage` Other 1.0)
      (`self.K2_DestroyActor`))
    (:`CastFailed`
      (cast `/Game/My/Character/BP_Bullet` Other
        (:`then`
          (`self.K2_DestroyActor`))
        (:`CastFailed`
          (bind _result (`/Engine/EditorBlueprintResources/StandardMacros.IncrementInt` (`self.HitNum`))
            (:`  `
              (bind _output_get (set `self.HitNum` _result))
              (if (== _output_get 2)
                (`self.K2_DestroyActor`)))))))))

(fn `UserConstructionScript`)