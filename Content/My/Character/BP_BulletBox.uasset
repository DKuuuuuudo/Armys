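; BP_BulletBox is an ammo pickup that restores a player's bullet count when a MyCharacter overlaps its Box trigger.
; The overlap sets AllBulletNum on that character's MyPlayerState to a fixed amount, then hides the ammo mesh and disables the box collision.
; A Respawn event waits a few seconds, then shows the mesh and re-enables collision through cached component references, making the pickup reusable.
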(event `self.Box.OnComponentBeginOverlap`
  (params (OverlappedComponent :type "PrimitiveComponent Object Reference") (OtherActor :type "Actor Object Reference") (OtherComp :type "PrimitiveComponent Object Reference") (OtherBodyIndex :type Integer) (bFromSweep :type Boolean) (SweepResult :type "HitResult Structure (by ref)"))
  (bind _sm_ammo (`self.SM_Ammo`))
  (bind _box (`self.Box`))
  (bind _asmy_character (cast `/Game/My/Character/MyCharacter` OtherActor))
  (bind _asmy_player_state (cast `/Game/My/Class/Main/MyPlayerState` (`Pawn.PlayerState` _asmy_character)))
  (set `/Game/My/Class/Main/MyPlayerState.AllBulletNum` 30 _asmy_player_state)
  (set `self.Temp_SM Ammo` _sm_ammo)
  (`SceneComponent.SetVisibility` _sm_ammo false false)
  (set `self.Temp_Box` _box)
  (`PrimitiveComponent.SetCollisionEnabled` _box "NoCollision")
  (`self.Respawn`))

(event `Respawn`
  (`KismetSystemLibrary.Delay` 5.0)
  (`SceneComponent.SetVisibility` (`self.Temp_SM Ammo`) true false)
  (`PrimitiveComponent.SetCollisionEnabled` (`self.Temp_Box`) "QueryAndPhysics"))

(fn `UserConstructionScript`)